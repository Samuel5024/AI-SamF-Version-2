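; Base enemy character Blueprint that provides attack, patrol route and movement speed functions.
; Attack plays the fire montage on the mesh, then calls OnAttackEnd and prints a debug message whether the montage completes or is interrupted.
; GetPatrolRoute exposes the stored route, and SetMovementSpeed maps a movement state from idle to sprinting onto the character's max walk speed and returns it.
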(event `self.ReceiveBeginPlay`)

(event `Attack`
  (`|PlayMontage` (`self.Mesh`) "/Game/Animations/Rifle/Gun/AM_Fire.AM_Fire"
    (:`OnCompleted`
      _)
    (:`OnInterrupted`
      _))
  (`self.OnAttackEnd`)
  (`KismetSystemLibrary.PrintString` "Attack Done"))

(fn `GetPatrolRoute`
  (returns (PatrolRoute :type "/Game/Enemies/AI/BP_PatrolRoute Object Reference"))
  (return (`self.PatrolRoute`)))

(fn `SetMovementSpeed`
  (params (Speed :type "/Game/Enemies/AI/Enums/E_MovementSpeed Enum" :default "NewEnumerator0"))
  (returns (SpeedValue :type "Float (double-precision)"))
  (bind _output_get (set `CharacterMovementComponent.MaxWalkSpeed` (select `/Game/Enemies/AI/Enums/E_MovementSpeed` Speed :`NewEnumerator1` 100.0 :`NewEnumerator2` 300.0 :`NewEnumerator3` 500.0 :!type "Float (single-precision)") (`self.CharacterMovement`)))
  (return _output_get))

(fn `UserConstructionScript`)